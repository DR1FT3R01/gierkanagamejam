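; BP_Arrow is an arrow actor, likely a rhythm game note, that moves vertically at a BPM-driven speed.
; Tick offsets it along world Z by DeltaSeconds and a BPM-derived value, then calls InWhichColumn.
; InWhichColumn maps world X bands to ColumnNumber for three columns; the fourth band's branch is empty.
; The below-line height check and actor hiding are unwired, and IsUnderLine is a stub.
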(event `self.ReceiveBeginPlay`)

(event `self.ReceiveTick`
  (params (DeltaSeconds :type "Float (single-precision)"))
  ;[1 1 1] Poruszanie się do bpm
  (bind _result (`/Engine/EditorBlueprintResources/StandardMacros.NegateFloat` (* DeltaSeconds (`self.BPM`)))
    (:`  `
      (`self.K2_AddActorWorldOffset` (`KismetMathLibrary.MakeVector` 0.0 0.0 _result))
      ;[1 1 1] Check która kolumna
      (`self.InWhichColumn` self))))

(fn `InWhichColumn`
  (returns (`Column Number` :type Integer))
  (bind _returnvalue_x (`KismetMathLibrary.BreakVector` (`self.K2_GetActorLocation` self)))
  (if (`KismetMathLibrary.InRange_FloatFloat` _returnvalue_x 500.0 600.0 true false)
    (set `self.Column Number` 0)
    (return (`self.Column Number`))
    (elif (`KismetMathLibrary.InRange_FloatFloat` _returnvalue_x 600.0 700.0 true false)
      (set `self.Column Number` 1)
      (return (`self.Column Number`))
      (elif (`KismetMathLibrary.InRange_FloatFloat` _returnvalue_x 700.0 800.0 true false)
        (set `self.Column Number` 2)
        (return (`self.Column Number`))
        (elif (`KismetMathLibrary.InRange_FloatFloat` _returnvalue_x 800.0 900.0)
          _)))))

(fn `IsUnderLine`
  (params (IsUnderLine :type Boolean)))

(fn `UnderLineCheck`
  (returns (IsUnderLine :type Boolean))
  (bind (_returnvalue_x _returnvalue_y _returnvalue_z) (`KismetMathLibrary.BreakVector` (`self.K2_GetActorLocation` self)))
  (return (< _returnvalue_z 100.0)))

(fn `UserConstructionScript`)