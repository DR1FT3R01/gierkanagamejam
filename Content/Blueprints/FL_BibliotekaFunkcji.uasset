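; Blueprint function library of small, partly unfinished gameplay helpers with Polish names, covering tile matching, a special check and HP.
; KtoryKafelek ("which tile") tests whether two resources equal a given ordered pair, and DodajHP returns HP plus one.
; CzySpecjalny ("is special") only stores the player pawn cast to Minicypek_BP; its tile-check logic is unconnected and returns nothing.
; NewFunction_0 is an empty stub.
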(fn `CzySpecjalny`
  (params (NewParam :type Integer))
  (locals (`Player Ref` :type "/Game/Blueprints/Minicypek_BP Object Reference"))
  (bind _asminicypek_bp (cast `/Game/Blueprints/Minicypek_BP` (`GameplayStatics.GetPlayerPawn` (`local.__WorldContext`))))
  (set `local.Player Ref` _asminicypek_bp))

(fn `DodajHP`
  (params (HP :type Integer))
  (returns (NoweHP :type Integer))
  (return (+ HP 1)))

(fn `KtoryKafelek`
  (params (`First Resource` :type Integer) (`Second Resource` :type Integer) (X :type Integer) (Y :type Integer))
  (returns (CzyKtoryKafelek :type Boolean))
  (return (and (== `First Resource` X) (== Y `Second Resource`))))

(fn `NewFunction_0`)