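; BP_Arrows is an arrow actor that moves along world Z each Tick, scaled by BPM, apparently for a rhythm mechanic.
; It also holds Money and Energy helpers and classifies diagonals by which pairs of directional resources are zero.
; Viability checks require positive Cooldown and map diagonals to rewards: upper-left money, lower-right energy (with a money minimum), the other two damage.
; The graphs shown never call these checks or counters.
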(event `self.ReceiveBeginPlay`)

(event `self.ReceiveTick`
  (params (DeltaSeconds :type "Float (single-precision)"))
  ;[1 1 1] Poruszanie się do bpm
  (bind _result (`/Engine/EditorBlueprintResources/StandardMacros.NegateFloat` (* DeltaSeconds (`self.BPM`)))
    (:`  `
      (`self.K2_AddActorWorldOffset` (`KismetMathLibrary.MakeVector` 0.0 0.0 _result)))))

(fn `AddEnergy`
  (set `self.Energy` (+ 1 (`self.Energy`))))

(fn `AddMoney`
  (set `self.Money` (+ (`self.Money`) 5)))

(fn `BPMFunction`
  (params (BPM :type "Float (double-precision)"))
  (returns (Delay :type "Float (double-precision)"))
  (bind _output_get (set `self.BPM` BPM))
  (return (/ (/ 60.0 (/ _output_get 60.0)) 100.0)))

(fn `EnergyCheck`
  (returns (IsEnergyHighierThan0 :type Boolean))
  (return (> (`self.Energy`) 0)))

(fn `IsLowerLeft`
  (returns (IsLowerLeft :type Boolean))
  (return (and (== (`self.Left Resource`) 0) (== 0 (`self.Down Resource`)))))

(fn `IsLowerRight`
  (returns (IsLowerRight :type Boolean))
  (return (and (== (`self.Right Resource`) 0) (== 0 (`self.Down Resource`)))))

(fn `IsSpecial`
  (returns (IsSpecial :type Boolean))
  (return (or (or (`self.IsLowerRight`) (`self.IsLowerLeft`)) (or (`self.IsUpperRight`) (`self.IsUpperLeft`)))))

(fn `IsUpperLeft`
  (returns (IsUpperLeft :type Boolean))
  (return (and (== (`self.Up Resource`) 0) (== 0 (`self.Left Resource`)))))

(fn `IsUpperRight`
  (returns (IsUpperRight :type Boolean))
  (return (and (== (`self.Up Resource`) 0) (== 0 (`self.Right Resource`)))))

(fn `IsViableDMG`
  (returns (IsCooldown :type Boolean))
  (return (and (> (`self.Cooldown`) 0) (or (`self.IsUpperRight`) (`self.IsLowerLeft`)))))

(fn `IsViableEnergy`
  (returns (IsViableEnergy :type Boolean))
  (return (and (> (`self.Cooldown`) 0) (and (`self.IsLowerRight`) (>= (`self.Money`) 5)))))

(fn `IsViableMoney`
  (returns (IsViableMoney :type Boolean))
  (return (and (> (`self.Cooldown`) 0) (`self.IsUpperLeft`))))

(fn `SubtractEnergy`
  (set `self.Energy` (- (`self.Energy`) 1)))

(fn `SubtractMoney`
  (set `self.Money` (- (`self.Money`) 5)))

(fn `UserConstructionScript`)