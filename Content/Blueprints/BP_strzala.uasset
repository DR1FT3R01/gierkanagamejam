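; BP_strzala spawns rows of four randomly rotated BP_Arrows across fixed columns, apparently for a rhythm game.
; BeginPlay runs the spawn body ten times without waiting, and its Delay loops back to keep spawning indefinitely.
; ArrowDelay sets the interval as BPM divided by 60, rather than seconds per beat.
; Tick is empty, leaving BPM movement, column detection and hiding logic disconnected.
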(event `self.ReceiveBeginPlay`
  (for _ (range 1 11)
    (`|SpawnActorFromClass` "/Game/Blueprints/BP_Arrows.BP_Arrows_C" (`KismetMathLibrary.MakeTransform` (550.0 -200.0 450.0) (`self.Randomize Rotation`)) "Undefined" "OverrideRootScale" null null :!label _label)
    (`|SpawnActorFromClass` "/Game/Blueprints/BP_Arrows.BP_Arrows_C" (`KismetMathLibrary.MakeTransform` (650.0 -200.0 450.0) (`self.Randomize Rotation`)) "Undefined" "OverrideRootScale" null null)
    (`|SpawnActorFromClass` "/Game/Blueprints/BP_Arrows.BP_Arrows_C" (`KismetMathLibrary.MakeTransform` (750.0 -200.0 450.0) (`self.Randomize Rotation`)) "Undefined" "OverrideRootScale" null null)
    (`|SpawnActorFromClass` "/Game/Blueprints/BP_Arrows.BP_Arrows_C" (`KismetMathLibrary.MakeTransform` (850.0 -200.0 450.0) (`self.Randomize Rotation`)) "Undefined" "OverrideRootScale" null null)
    (`KismetSystemLibrary.Delay` (`self.ArrowDelay` 130.0))
    (goto _label)))

(event `self.ReceiveTick`
  (params (DeltaSeconds :type "Float (single-precision)")))

(fn `ArrowDelay`
  (params (BPM :type "Float (double-precision)"))
  (returns (Delay :type "Float (double-precision)"))
  (bind _output_get (set `self.BPM` BPM))
  (return (/ _output_get 60.0)))

(fn `InWhichColumn`
  (returns (`Column Number` :type Integer))
  (bind _returnvalue_x (`KismetMathLibrary.BreakVector` (`self.K2_GetActorLocation` self)))
  (if (`KismetMathLibrary.InRange_FloatFloat` _returnvalue_x 500.0 600.0 true false)
    (set `self.Column Number` 0)
    (return (`self.Column Number`))
    (elif (`KismetMathLibrary.InRange_FloatFloat` _returnvalue_x 600.0 700.0 true false)
      (set `self.Column Number` 1)
      (return (`self.Column Number`))
      (elif (`KismetMathLibrary.InRange_FloatFloat` _returnvalue_x 700.0 800.0 true false)
        (set `self.Column Number` 2)
        (return (`self.Column Number`))
        (elif (`KismetMathLibrary.InRange_FloatFloat` _returnvalue_x 800.0 900.0)
          (set `self.Column Number` 3)
          (return (`self.Column Number`)))))))

(fn `IsUnderLine`
  (params (IsUnderLine :type Boolean)))

(fn `Randomize Rotation`
  (returns (RandomizedRotation :type "Rotator Structure"))
  (switch `int` (`KismetMathLibrary.RandomIntegerInRange` 0 3)
    (:`0`
      (set `self.ArrowRotation` (struct)))
    (:`1`
      (set `self.ArrowRotation` (struct :`Pitch` 90.0)))
    (:`2`
      (set `self.ArrowRotation` (struct :`Pitch` 180.0)))
    (:`3`
      (set `self.ArrowRotation` (struct :`Pitch` 270.0))))
  (return (`self.ArrowRotation`)))

(fn `UnderLineCheck`
  (returns (IsUnderLine :type Boolean))
  (bind (_returnvalue_x _returnvalue_y _returnvalue_z) (`KismetMathLibrary.BreakVector` (`self.K2_GetActorLocation` self)))
  (return (< _returnvalue_z 100.0)))

(fn `UserConstructionScript`)