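; Player Blueprint that moves in 100-unit steps on the X/Z plane while managing Money and Energy.
; Each move spends that direction's resource and refunds the opposite one, confining movement to a 3x3 grid around the start.
; Tick checks for a special state, applying money gain, money-for-energy exchange or energy damage, gated by helper checks and a Cooldown flag.
; A failed energy check afterwards quits the game; UI widget creation is unconnected.
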(event `self.ReceiveBeginPlay`
  (set `self.Up Resource` 1)
  (set `self.Down Resource` 1)
  (set `self.Left Resource` 1)
  (set `self.Right Resource` 1)
  (set `self.Energy` 20)
  (set `self.Money` 20))

(event `Key|Down`
  (params (Key :type "Key Structure"))
  ;[1 1 1] Movement
  (:`Pressed`
    (if (> (`self.Down Resource`) 0)
      (`self.K2_AddActorWorldOffset` (0.0 0.0 -100.0))
      (`/Engine/EditorBlueprintResources/StandardMacros.DecrementInt` (`self.Down Resource`)
        (:`  `
          (`/Engine/EditorBlueprintResources/StandardMacros.IncrementInt` (`self.Up Resource`)))))))

(event `Key|Up`
  (params (Key :type "Key Structure"))
  ;[1 1 1] Movement
  (:`Pressed`
    (if (> (`self.Up Resource`) 0)
      (`self.K2_AddActorWorldOffset` (0.0 0.0 100.0))
      (`/Engine/EditorBlueprintResources/StandardMacros.DecrementInt` (`self.Up Resource`)
        (:`  `
          (`/Engine/EditorBlueprintResources/StandardMacros.IncrementInt` (`self.Down Resource`)))))))

(event `Key|Left`
  (params (Key :type "Key Structure"))
  ;[1 1 1] Movement
  (:`Pressed`
    (if (> (`self.Left Resource`) 0)
      (`self.K2_AddActorWorldOffset` (-100.0 0.0 0.0))
      (`/Engine/EditorBlueprintResources/StandardMacros.DecrementInt` (`self.Left Resource`)
        (:`  `
          (`/Engine/EditorBlueprintResources/StandardMacros.IncrementInt` (`self.Right Resource`)))))))

(event `Key|Right`
  (params (Key :type "Key Structure"))
  ;[1 1 1] Movement
  (:`Pressed`
    (if (> (`self.Right Resource`) 0)
      (`self.K2_AddActorWorldOffset` (100.0 0.0 0.0))
      (`/Engine/EditorBlueprintResources/StandardMacros.DecrementInt` (`self.Right Resource`)
        (:`  `
          (`/Engine/EditorBlueprintResources/StandardMacros.IncrementInt` (`self.Left Resource`)))))))

(event `self.ReceiveTick`
  (params (DeltaSeconds :type "Float (single-precision)"))
  (if (`self.IsSpecial`)
    (if (`self.IsViableMoney`)
      (`self.AddMoney`)
      (set `self.Cooldown` 0)
      (`KismetSystemLibrary.PrintString` (`KismetStringLibrary.Conv_IntToString` (`self.Money`)))
      (`KismetSystemLibrary.PrintString` "Money:")
      (if (not (`self.EnergyCheck`)) :!label _label
        (`self.K2_DestroyActor` self)
        (`KismetSystemLibrary.QuitGame` null "Quit"))
      (elif (`self.IsViableEnergy`)
        (`self.SubtractMoney`)
        (`self.AddEnergy`)
        (set `self.Cooldown` 0)
        (`KismetSystemLibrary.PrintString` (`KismetStringLibrary.Conv_IntToString` (`self.Energy`)))
        (`KismetSystemLibrary.PrintString` "Energy:")
        (goto _label)
        (elif (`self.IsViableDMG`)
          (`self.SubtractEnergy`)
          (set `self.Cooldown` 0)
          (`KismetSystemLibrary.PrintString` (`KismetStringLibrary.Conv_IntToString` (`self.Energy`)))
          (`KismetSystemLibrary.PrintString` "DMG")
          (goto _label))))
    (else
      (set `self.Cooldown` 1))))

(fn `UserConstructionScript`
  (`parent.UserConstructionScript`))