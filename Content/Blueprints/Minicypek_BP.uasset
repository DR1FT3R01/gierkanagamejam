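; Minicypek is a key-controlled actor that steps in 100-unit jumps on the X/Z plane within a 3x3 grid around its start.
; Paired directional counters act as bounds, with each step spending one direction's counter and refunding its opposite.
; While it sits in the bottom-right cell, Tick trades Sianogrosze for EnergyLandia2000 every frame until funds run short, printing both values.
; The overlap event and CzyMackaStyka function are empty.
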(event `self.ReceiveBeginPlay`
  (set `self.UpResource` 1)
  (set `self.DownResource` 1)
  (set `self.LeftResource` 1)
  (set `self.RightResource` 1)
  (set `self.EnergyLandia2000` 100)
  (set `self.Sianogrosze` 20))

(event `Key|Down`
  (params (Key :type "Key Structure"))
  ;[1 1 1] Movement
  (:`Pressed`
    (if (> (`self.DownResource`) 0)
      (`self.K2_AddActorWorldOffset` (0.0 0.0 -100.0))
      (`/Engine/EditorBlueprintResources/StandardMacros.DecrementInt` (`self.DownResource`)
        (:`  `
          (`/Engine/EditorBlueprintResources/StandardMacros.IncrementInt` (`self.UpResource`)))))))

(event `Key|Up`
  (params (Key :type "Key Structure"))
  ;[1 1 1] Movement
  (:`Pressed`
    (if (> (`self.UpResource`) 0)
      (`self.K2_AddActorWorldOffset` (0.0 0.0 100.0))
      (`/Engine/EditorBlueprintResources/StandardMacros.DecrementInt` (`self.UpResource`)
        (:`  `
          (`/Engine/EditorBlueprintResources/StandardMacros.IncrementInt` (`self.DownResource`)))))))

(event `Key|Left`
  (params (Key :type "Key Structure"))
  ;[1 1 1] Movement
  (:`Pressed`
    (if (> (`self.LeftResource`) 0)
      (`self.K2_AddActorWorldOffset` (-100.0 0.0 0.0))
      (`/Engine/EditorBlueprintResources/StandardMacros.DecrementInt` (`self.LeftResource`)
        (:`  `
          (`/Engine/EditorBlueprintResources/StandardMacros.IncrementInt` (`self.RightResource`)))))))

(event `Key|Right`
  (params (Key :type "Key Structure"))
  ;[1 1 1] Movement
  (:`Pressed`
    (if (> (`self.RightResource`) 0)
      (`self.K2_AddActorWorldOffset` (100.0 0.0 0.0))
      (`/Engine/EditorBlueprintResources/StandardMacros.DecrementInt` (`self.RightResource`)
        (:`  `
          (`/Engine/EditorBlueprintResources/StandardMacros.IncrementInt` (`self.LeftResource`)))))))

(event `self.ReceiveTick`
  (params (DeltaSeconds :type "Float (single-precision)"))
  (if (and (and (== (`self.RightResource`) 0) (== 0 (`self.DownResource`))) (>= (`self.Sianogrosze`) 5))
    (set `self.Sianogrosze` (- (`self.Sianogrosze`) 5))
    (bind _output_get (set `self.EnergyLandia2000` (+ 2 (`self.EnergyLandia2000`))))
    (`KismetSystemLibrary.PrintString` (`KismetStringLibrary.Conv_IntToString` _output_get))
    (`KismetSystemLibrary.PrintString` (`KismetStringLibrary.Conv_IntToString` (`self.Sianogrosze`)))))

(fn `CzyMackaStyka`)

(fn `UserConstructionScript`)